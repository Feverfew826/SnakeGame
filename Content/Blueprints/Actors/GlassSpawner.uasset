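; GlassSpawner is an actor that scatters clumps of grass static meshes inside its SpawnVolume box, built entirely in the Construction Script.
; It picks GrassNumber random chunk centers, inset from the box edges, then adds GrassChunkSize mesh components around each at random flat offsets and yaw.
; Mesh scale divides out actor scale, keeping blades a constant, half-height size.
; Randomness is unseeded, and event graph nodes are empty.
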(event EventBeginPlay)

(event Collision|EventActorBeginOverlap
  (params (OtherActor :type Actor%20Object%20Reference)))

(event EventTick
  (params (DeltaSeconds :type Float%20%28single-precision%29)))

(fn ConstructionScript
  (bind _returnvalue (Math|Vector|MakeVector 0.0 0.0 0.0))
  (bind _returnvalue_2 (Math|Vector|MakeVector 1.0 1.0 0.5))
  (bind _returnvalue_3 (Math|Random|RandomUnitVector))
  (bind _returnvalue_4 (Transformation|GetActorScale3D))
  (bind _spawnvolume (Variables|Default|GetSpawnVolume))
  (bind _grasschunksize (LocalVariables|GetGrassChunkSize))
  (bind _eachgrassoffset (LocalVariables|GetEachGrassOffset))
  (bind _returnvalue_5 (Components|Box|GetUnscaledBoxExtent _spawnvolume))
  (bind _returnvalue_6 (* _grasschunksize _eachgrassoffset))
  (bind (_x _y) (Math|Vector|BreakVector _returnvalue_3))
  (bind _returnvalue_7 (- _returnvalue_5 _returnvalue_6))
  (bind _returnvalue_8 (Math|Random|RandomPointinBoundingBox _returnvalue _returnvalue_7))
  (for _index (range 1 (Variables|Default|GetGrassNumber))
    (LocalVariables|SetGrassChunkPosition (Math|Vector|MakeVector (.x _returnvalue_8) (.y _returnvalue_8) 0.0))
    (for _index_2 (range 1 (LocalVariables|GetGrassChunkSize))
      (AddComponent|AddStaticMeshComponent false (Math|Transform|MakeTransform (+ (LocalVariables|GetGrassChunkPosition) (* (Math|Vector|MakeVector _x _y 0.0) (Math|Random|RandomFloatinRange 0.0 (* (LocalVariables|GetGrassChunkSize) (LocalVariables|GetEachGrassOffset))))) (Math|Rotator|MakeRotator 0.0 0.0 (Math|Random|RandomFloatinRange 0.0 3.6e+02)) (Math|Vector|MakeVector (/ (.x _returnvalue_2) (.x _returnvalue_4)) (/ (.y _returnvalue_2) (.y _returnvalue_4)) (/ (.z _returnvalue_2) (.z _returnvalue_4))))))))