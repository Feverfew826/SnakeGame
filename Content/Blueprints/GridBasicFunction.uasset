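; Blueprint function library of grid math helpers for movement in four directions on the X/Y plane.
; CalcNextPosition steps the moving axis to the adjacent grid line and snaps the other axes with SnapVectorToGrid, with Up as negative Y and Right as positive X.
; Floor-plus-one and Ceil-minus-one rounding makes each step land strictly past the current value, even when off-grid.
; CalcRotator maps each direction to a matching right-angle rotation.
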(fn SnapVectortoGrid
  (params (InputVector :type Vector) (GridSize :type Integer))
  (return (Math|Vector|MakeVector (Math|Float|SnapToGrid(Float) (.x InputVector) (Math|Conversions|ToFloat(Integer) GridSize)) (Math|Float|SnapToGrid(Float) (.y InputVector) (Math|Conversions|ToFloat(Integer) GridSize)) (Math|Float|SnapToGrid(Float) (.z InputVector) (Math|Conversions|ToFloat(Integer) GridSize)))))

(fn CalcRotator
  (params (Direction :type EDirection4%20Enum :default "NewEnumerator0"))
  (return (Utilities|Select :Index Direction :NewEnumerator0 "0,270.000000, 0" :NewEnumerator1 "0.000000,90.000000,0.000000" :NewEnumerator2 "0.000000,180.000000,0.000000" :NewEnumerator3 "0, 0, 0")))

(fn CalcNextPosition
  (params (CurrentPosition :type Vector) (Direction :type EDirection4%20Enum :default "NewEnumerator0") (GridSize :type Integer))
  (bind _returnvalue (Math|Vector|MakeVector (.x CurrentPosition) (.y CurrentPosition) (.z CurrentPosition)))
  (bind _returnvalue_2 (Math|Vector|MakeVector (.x CurrentPosition) (.y CurrentPosition) (.z CurrentPosition)))
  (bind _returnvalue_3 (Math|Vector|MakeVector (.x CurrentPosition) (.y CurrentPosition) (.z CurrentPosition)))
  (bind _returnvalue_4 (Math|Vector|MakeVector (.x CurrentPosition) (.y CurrentPosition) (.z CurrentPosition)))
  (bind _returnvector (CallFunction|SnapVectortoGrid _returnvalue GridSize))
  (bind _returnvector_2 (CallFunction|SnapVectortoGrid _returnvalue_3 GridSize))
  (bind _returnvector_3 (CallFunction|SnapVectortoGrid _returnvalue_4 GridSize))
  (bind _returnvector_4 (CallFunction|SnapVectortoGrid _returnvalue_2 GridSize))
  (return (Utilities|Select :Index Direction :NewEnumerator0 (Math|Vector|MakeVector (.x _returnvector) (CallFunction|CalcPreviousGridValue (.y CurrentPosition) GridSize) (.z _returnvector)) :NewEnumerator1 (Math|Vector|MakeVector (.x _returnvector_2) (CallFunction|CalcNextGridValue (.y CurrentPosition) GridSize) (.z _returnvector_2)) :NewEnumerator2 (Math|Vector|MakeVector (CallFunction|CalcPreviousGridValue (.x CurrentPosition) GridSize) (.y _returnvector_3) (.z _returnvector_3)) :NewEnumerator3 (Math|Vector|MakeVector (CallFunction|CalcNextGridValue (.x CurrentPosition) GridSize) (.y _returnvector_4) (.z _returnvector_4)))))

(fn CalcNextGridValue
  (params (A :type Float%20%28single-precision%29) (GridSize :type Integer))
  (return (Math|Conversions|ToFloat(Integer) (* (+ (Math|Float|Floor (/ A (Math|Conversions|ToFloat(Integer) GridSize))) 1) GridSize))))

(fn CalcPreviousGridValue
  (params (A :type Float%20%28single-precision%29) (GridSize :type Integer))
  (return (Math|Conversions|ToFloat(Integer) (* (- (Math|Float|Ceil (/ A (Math|Conversions|ToFloat(Integer) GridSize))) 1) GridSize))))