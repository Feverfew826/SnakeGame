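; Grid movement component that slides its owning actor one cell at a time in four directions on the XY plane.
; MoveToNextPosition snaps the start to the grid, then Tick lerps toward the target cell by clamped game time over MoveDuration.
; On arrival it calls OnReachedTargetPosition, leaving ShouldMove true.
; Helpers snap positions and pick a step direction toward a target, checking Y before X.
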(event Custom|MoveToNextPosition
  (params (Direction :type EDirection4%20Enum :default "NewEnumerator0"))
  (Variables|Movement|SetStartPosition (PureFunction|SnapVectortoGrid (Transformation|GetActorLocation (Components|GetOwner)) (Variables|GridMovementOption|GetGridSize)))
  (Variables|Movement|SetTargetDirection Direction)
  (Variables|Movement|SetStartGameTime (Utilities|Time|GetGameTimeinSeconds))
  (Variables|Default|SetShouldMove true))

(event EventBeginPlay
  (Variables|Movement|SetStartPosition (Transformation|GetActorLocation (Components|GetOwner))))

(event EventTick
  (params (DeltaSeconds :type Float%20%28single-precision%29))
  (bind _returnvalue (Utilities|Time|GetGameTimeinSeconds))
  (bind _moveduration (Variables|GridMovementOption|GetMoveDuration))
  (bind _startgametime (Variables|Movement|GetStartGameTime))
  (bind _passedtimerate (PureFunction|CalcTimeRate _returnvalue _startgametime _moveduration))
  (if (Variables|Default|GetShouldMove)
    (Transformation|SetActorLocation (Components|GetOwner) (Math|Vector|Lerp(Vector) (Variables|Movement|GetStartPosition) (Utilities|GetTargetPosition) _passedtimerate) false false)
    (if (>= _passedtimerate 1.0)
      (Variables|Default|SetShouldMove true)
      (Default|CallOnReachedTargetPosition))))

(fn SnapActortoGrid
  (params (TargetActor :type Actor%20Object%20Reference) (GridSize :type Integer))
  (Transformation|SetActorLocation TargetActor (PureFunction|SnapVectortoGrid (Transformation|GetActorLocation TargetActor) GridSize) false false))

(fn SnapVectortoGrid
  (params (InputVector :type Vector) (GridSize :type Integer))
  (return (Math|Vector|MakeVector (Math|Float|SnapToGrid(Float) (.x InputVector) (Math|Conversions|ToFloat(Integer) GridSize)) (Math|Float|SnapToGrid(Float) (.y InputVector) (Math|Conversions|ToFloat(Integer) GridSize)) (Math|Float|SnapToGrid(Float) (.z InputVector) (Math|Conversions|ToFloat(Integer) GridSize)))))

(fn CalcNextPosition
  (params (CurrentPosition :type Vector) (Direction :type EDirection4%20Enum :default "NewEnumerator0") (GridSize :type Integer))
  (return (+ CurrentPosition (PureFunction|CalcNextDistance Direction GridSize))))

(fn CalcNextDistance
  (params (Direction :type EDirection4%20Enum :default "NewEnumerator0") (GridSize :type Integer))
  (switch Utilities|FlowControl|Switch|SwitchonEDirection4 Direction
    (:NewEnumerator0
      (return (Math|Vector|MakeVector 0.0 (* GridSize -1.0) 0.0)))
    (:NewEnumerator1
      (return (Math|Vector|MakeVector 0.0 (Math|Conversions|ToFloat(Integer) GridSize) 0.0)))
    (:NewEnumerator2
      (return (Math|Vector|MakeVector (* GridSize -1.0) 0.0 0.0)))
    (:NewEnumerator3
      (return (Math|Vector|MakeVector (Math|Conversions|ToFloat(Integer) GridSize) 0.0 0.0)))))

(fn CalcTimeRate
  (params (CurrentGameTime :type Float%20%28single-precision%29) (StartGameTime :type Float%20%28single-precision%29) (Duration :type Float%20%28single-precision%29))
  (return (Math|Float|Clamp(Float) (/ (- CurrentGameTime StartGameTime) Duration))))

(fn CalcTargetDirection
  (params (StartPosition :type Vector) (Target :type Vector) (GridSize :type Integer))
  (bind _returnvector (PureFunction|SnapVectortoGrid StartPosition GridSize))
  (bind _returnvector_2 (PureFunction|SnapVectortoGrid Target GridSize))
  (if (> (.y _returnvector) (.y _returnvector_2))
    (return true "NewEnumerator0")
    (elif (< (.y _returnvector) (.y _returnvector_2))
      (return true "NewEnumerator1")
      (elif (< (.x _returnvector) (.x _returnvector_2))
        (return true "NewEnumerator3")
        (elif (> (.x _returnvector) (.x _returnvector_2))
          (return true "NewEnumerator2")
          (else
            (return false "NewEnumerator0")))))))