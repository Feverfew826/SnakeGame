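; GridMovement2 is a component that moves its owning actor in grid steps at a constant speed.
; MoveToNextPosition stores a direction and starts movement.
; While moving, Tick recomputes the target with CalcNextPosition from current location, direction and grid size, then applies VInterpToConstant without sweep.
; When the interpolated location matches the target, it stops and calls OnReachedNextPosition.
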(event Custom|MoveToNextPosition
  (params (Direction :type EDirection4%20Enum :default "NewEnumerator0"))
  (Variables|Default|SetDirection Direction)
  (Variables|Default|SetShouldMove true))

(event EventBeginPlay)

(event EventTick
  (params (DeltaSeconds :type Float%20%28single-precision%29))
  (bind _returnvalue (Components|GetOwner))
  (bind _gridsize (Variables|Default|GetGridSize))
  (bind _direction (Variables|Default|GetDirection))
  (bind _speed (Variables|Default|GetSpeed))
  (bind _returnvalue_2 (Transformation|GetActorLocation _returnvalue))
  (bind _nextposition (CallFunction|CalcNextPosition _returnvalue_2 _direction _gridsize))
  (bind _returnvalue_3 (Math|Interpolation|VInterptoConstant _returnvalue_2 _nextposition DeltaSeconds _speed))
  (if (Variables|Default|GetShouldMove)
    (Transformation|SetActorLocation (Components|GetOwner) _returnvalue_3 false false)
    (if (Math|Vector|Equal(Vector) _returnvalue_3 _nextposition 0.0001)
      (Variables|Default|SetShouldMove false)
      (Default|CallOnReachedNextPosition))))