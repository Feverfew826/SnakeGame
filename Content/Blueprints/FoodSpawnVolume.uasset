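; FoodSpawnVolume is an actor that keeps a single Food item present inside its SpawnVolume box.
; On BeginPlay it spawns Food at a random point within the box, snapped to a 100-unit grid and spawned regardless of collision.
; It binds to that Food's OnDestroyed event, so each destruction immediately spawns a replacement at a new random grid position.
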(event Custom|SpawnFood
  (bind _spawnvolume (Variables|Default|GetSpawnVolume))
  (bind _returnvalue (Game|SpawnActorfromClass "/Game/Blueprints/Food.Food_C" (Math|Conversions|ToTransform(Vector) (CallFunction|SnapVectortoGrid (Math|Random|RandomPointinBoundingBox (Transformation|GetWorldLocation _spawnvolume) (Components|Box|GetScaledBoxExtent _spawnvolume)) 100)) "AlwaysSpawn" 0 0))
  (Game|BindEventtoOnDestroyed _returnvalue (delegate Custom|FoodDestroyed)))

(event Custom|FoodDestroyed
  (params (DestroyedActor :type Actor%20Object%20Reference))
  (CallFunction|SpawnFood))

(event EventBeginPlay
  (CallFunction|SpawnFood))

(event Collision|EventActorBeginOverlap
  (params (OtherActor :type Actor%20Object%20Reference)))

(event EventTick
  (params (DeltaSeconds :type Float%20%28single-precision%29)))

(fn ConstructionScript)